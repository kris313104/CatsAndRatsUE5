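; Dungeon generator for the first level that builds its room layout on BeginPlay by overriding the generator's rule functions.
; It starts from the starting room and adds random normal rooms, offering the final room once the minimum count is reached until one is placed.
; Growth stops at the maximum room count, and a layout is valid only with the final room.
; Connections between two rooms get doors, while open ends get walls.
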(event `self.ReceiveBeginPlay`
  (`self.Generate`))

(fn `ChooseDoor`
  (params (CurrentRoom :type "RoomData Object Reference") (NextRoom :type "RoomData Object Reference"))
  (returns (ReturnValue :type "Door Class Reference"))
  (if (and (`KismetSystemLibrary.IsValid` CurrentRoom) (`KismetSystemLibrary.IsValid` NextRoom))
    (return "/Game/Blueprints/Dungeon/Generator/FirstLevel/BP_FirstLevelDoor.BP_FirstLevelDoor_C")
    (else
      (return "/Game/Blueprints/Dungeon/Generator/FirstLevel/BP_FirstLevelWall.BP_FirstLevelWall_C"))))

(fn `ChooseFirstRoomData`
  (returns (ReturnValue :type "RoomData Object Reference"))
  (return (`self.StartingRoom`)))

(fn `ChooseNextRoomData`
  (params (CurrentRoom :type "RoomData Object Reference"))
  (returns (ReturnValue :type "RoomData Object Reference"))
  (if (and (>= (`self.GetNbRoom`) (`self.MinRooms`)) (not (`self.HasAlreadyRoomData` (`self.FinalRoom`))))
    (return (`self.FinalRoom`))
    (else
      (bind _returnvalue (`self.GetRandomRoomData` (`self.NormalRooms`)))
      (return _returnvalue))))

(fn `ContinueToAddRoom`
  (returns (ReturnValue :type Boolean))
  (return (< (`self.GetNbRoom`) (`self.MaxRooms`))))

(fn `IsValidDungeon`
  (returns (ReturnValue :type Boolean))
  (return (`self.HasAlreadyRoomData` (`self.FinalRoom`))))

(fn `UserConstructionScript`)