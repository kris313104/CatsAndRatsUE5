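; First-level dungeon generator Blueprint that builds a procedural room layout on BeginPlay by overriding the generator's room-selection and validation functions.
; Layouts start with SpawnRoom and draw random picks from NormalRooms, switching to ExitRoom once MinRooms is reached until an exit is placed.
; Rooms are added while the count is below MaxRooms, and a dungeon is valid only if it contains ExitRoom.
; Debug prints run during validation and after generation.
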(event `self.ReceiveBeginPlay`
  (`self.Generate`))

(event `self.OnPostGeneration_BP`
  (`KismetSystemLibrary.PrintString` "generated"))

(fn `ChooseFirstRoomData`
  (returns (ReturnValue :type "RoomData Object Reference"))
  (return (`self.SpawnRoom`)))

(fn `ChooseNextRoomData`
  (params (CurrentRoom :type "RoomData Object Reference"))
  (returns (ReturnValue :type "RoomData Object Reference"))
  (if (and (>= (`self.GetNbRoom`) (`self.MinRooms`)) (not (`self.HasAlreadyRoomData` (`self.ExitRoom`))))
    (return (`self.ExitRoom`))
    (else
      (bind _returnvalue (`self.GetRandomRoomData` (`self.NormalRooms`)))
      (return _returnvalue))))

(fn `ContinueToAddRoom`
  (returns (ReturnValue :type Boolean))
  (return (< (`self.GetNbRoom`) (`self.MaxRooms`))))

(fn `IsValidDungeon`
  (returns (ReturnValue :type Boolean))
  (bind _returnvalue (`self.HasAlreadyRoomData` (`self.ExitRoom`)))
  (`KismetSystemLibrary.PrintString` "Hello" _returnvalue)
  (return _returnvalue))

(fn `UserConstructionScript`)