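; Level transition trigger that loads the level named in LevelToTransitionTo when the player interacts with it.
; Entering TransitionRange sends interact-area messages to the overlapping actor and sets the BP_Hero message widget text to TransitionMessage.
; Leaving the range sends the exit message.
; DoInteraction prints a debug string, opens the level and sets game-only input.
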(event `self.TransitionRange.OnComponentBeginOverlap`
  (params (OverlappedComponent :type "PrimitiveComponent Object Reference") (OtherActor :type "Actor Object Reference") (OtherComp :type "PrimitiveComponent Object Reference") (OtherBodyIndex :type Integer) (bFromSweep :type Boolean) (SweepResult :type "HitResult Structure (by ref)"))
  (message `/Game/Blueprints/Messaging/BPI_InteractInterface.InteractAreaEntered` OtherActor self)
  (bind _asbp_hero (cast `/Game/Blueprints/Hero/BP_Hero` (`GameplayStatics.GetPlayerCharacter` 0)))
  (set `MessageUserWidget.Message` (`self.TransitionMessage`) (`/Game/Blueprints/Hero/BP_Hero.MessageUserWidget` _asbp_hero))
  (message `/Game/Blueprints/Messaging/BPI_InteractInterface.InteractAreaEntered` OtherActor null))

(event `self.TransitionRange.OnComponentEndOverlap`
  (params (OverlappedComponent :type "PrimitiveComponent Object Reference") (OtherActor :type "Actor Object Reference") (OtherComp :type "PrimitiveComponent Object Reference") (OtherBodyIndex :type Integer))
  (message `/Game/Blueprints/Messaging/BPI_InteractInterface.InteractAreaExited` OtherActor))

(event `/Game/Blueprints/Messaging/BPI_InteractInterface.DoInteraction`
  (`KismetSystemLibrary.PrintString` "Hello")
  (`GameplayStatics.OpenLevel` (`self.LevelToTransitionTo`))
  (`WidgetBlueprintLibrary.SetInputMode_GameOnly` (`GameplayStatics.GetPlayerController` 0)))

(fn `UserConstructionScript`)