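; Slime enemy Blueprint that feeds player detection to its AI and reacts to damage.
; Pawn sensing sets the HasSeenPlayer Blackboard key on spotting the Hero, and Tick clears it after a short delay once the player is beyond sight radius.
; Damage jumps the animation to Hurting, or at low health to Dying, disabling collision and sight and clearing IsEnemySelected on every Minion's Blackboard.
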(event `self.ReceiveTick`
  (params (DeltaSeconds :type "Float (single-precision)"))
  (if (> (`self.GetDistanceTo` (`GameplayStatics.GetPlayerPawn` 0) self) (`PawnSensingComponent.SightRadius` (`self.SensingComponent`)))
    (`KismetSystemLibrary.Delay` 0.5)
    (`BlackboardComponent.SetValueAsBool` (`AIBlueprintHelperLibrary.GetBlackboard` (`AIBlueprintHelperLibrary.GetAIController` self)) "HasSeenPlayer" false)))

(event `self.SensingComponent.OnSeePawn`
  (params (Pawn :type "Pawn Object Reference"))
  (cast `Hero` Pawn)
  (`BlackboardComponent.SetValueAsBool` (`AIBlueprintHelperLibrary.GetBlackboard` (`AIBlueprintHelperLibrary.GetAIController` self)) "HasSeenPlayer" true))

(event `self.ReceiveAnyDamage`
  (params (Damage :type "Float (single-precision)") (DamageType :type "DamageType Object Reference") (InstigatedBy :type "Controller Object Reference") (DamageCauser :type "Actor Object Reference"))
  (bind _animinstance (`PaperZDAnimationComponent.AnimInstance` (`self.AnimationComponent`)))
  (if (<= (`HealthComponent.CurrentHealth` (`self.HealthComponent`)) 1)
    (`PawnSensingComponent.SetSensingInterval` (`self.SensingComponent`) 0.0)
    (`PaperZDAnimInstance.JumpToNode` _animinstance "Dying" "None")
    (`PrimitiveComponent.SetCollisionEnabled` (`self.CapsuleComponent`) "NoCollision")
    (set `PawnSensingComponent.SightRadius` 0.0 (`self.SensingComponent`))
    (bind _outactors (`GameplayStatics.GetAllActorsOfClass` "/Script/CatsAndRats2D.Minion"))
    (for _array_element _outactors
      (`BlackboardComponent.SetValueAsBool` (`AIBlueprintHelperLibrary.GetBlackboard` _array_element) "IsEnemySelected" false))
    (else
      (`PaperZDAnimInstance.JumpToNode` _animinstance "Hurting" "None"))))

(fn `UserConstructionScript`)