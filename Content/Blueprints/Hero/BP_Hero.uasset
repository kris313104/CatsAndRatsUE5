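; Player hero Blueprint for a 2D game, handling weapon draw and sheathe, melee combos and the heart-based health UI.
; Tick plays draw or sheathe animations from IsDrawn while grounded, using JumpToNode and locking movement.
; Attack input advances AttackState, starting the first swing directly and signaling follow-ups through transition flags on the game mode.
; BeginPlay creates the main UI, and AnyDamage updates its hearts one step at a time.
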(event `self.ReceiveTick`
  (params (DeltaSeconds :type "Float (single-precision)"))
  (`|ExecutionSequence`
    (:`then_0`
      ;[1 1 1] draw
      (if (and (and (not (`NavMovementComponent.IsFalling` (`self.CharacterMovement`))) (not (`self.CanDrwSht`))) (`self.IsDrawn`))
        (set `self.CanDrwSht` true)
        (`PaperZDAnimInstance.JumpToNode` (`PaperZDAnimationComponent.AnimInstance` (`self.AnimationComponent`)) "Drawing" "None")
        (`MovementComponent.StopMovementImmediately` (`self.CharacterMovement`))
        (set `self.IsMovementLocked` true)))
    (:`then_1`
      ;[1 1 1] shite
      (if (and (and (not (`NavMovementComponent.IsFalling` (`self.CharacterMovement`))) (not (`self.CanDrwSht`))) (not (`self.IsDrawn`)))
        (set `self.CanDrwSht` true)
        (`PaperZDAnimInstance.JumpToNode` (`PaperZDAnimationComponent.AnimInstance` (`self.AnimationComponent`)) "Shiting" "None")
        (`MovementComponent.StopMovementImmediately` (`self.CharacterMovement`))
        (set `self.IsMovementLocked` true)))))

(event `self.ReceiveBeginPlay`
  (set `self.Animation Component` (`self.AnimationComponent`))
  (bind _returnvalue (`|CreateWidget` "/Game/Blueprints/UI/Hero/WBP_MainUI.WBP_MainUI_C"))
  (bind _output_get (set `self.MainUIRef` _returnvalue))
  (`UserWidget.AddToViewport` _output_get 0))

(event `self.ReceiveAnyDamage`
  (params (Damage :type "Float (single-precision)") (DamageType :type "DamageType Object Reference") (InstigatedBy :type "Controller Object Reference") (DamageCauser :type "Actor Object Reference"))
  (bind _result (`/Engine/EditorBlueprintResources/StandardMacros.NegateInt` (`KismetMathLibrary.FTrunc` Damage))
    (:`  `
      (for _ (range 1 (+ (`KismetMathLibrary.Abs_Int` _result) 1))
        (`/Game/Blueprints/UI/Hero/WBP_MainUI.UpdateHearts` (`self.MainUIRef`) (select `bool` (> _result 0) :`false` -1 :`true` 1))))))

(event `EnhancedInput|/Game/Input/Action/IA_Attack`
  (params (ActionValue :type Boolean) (ElapsedSeconds :type "Float (double-precision)") (TriggeredSeconds :type "Float (double-precision)") (InputAction :type "InputAction Object Reference" :default "/Game/Input/Action/IA_Attack.IA_Attack"))
  (:`Started`
    (if (== (`self.CanAttack`) true)
      (bind _result (`/Engine/EditorBlueprintResources/StandardMacros.IncrementInt` (`self.AttackState`))
        (:`  `
          (bind _output_get (set `self.AttackState` _result))
          (set `self.CanAttack` false)
          (if (== _output_get 4)
            (set `self.AttackState` 0)
            (bind _asbp_cats_and_rats_2dgame_mode_base (cast `/Game/Blueprints/GameMode/BP_CatsAndRats2DGameModeBase` (`GameplayStatics.GetGameMode`)))
            (`CatsAndRats2DGameModeBase.SetTransitionToNextAttack` _asbp_cats_and_rats_2dgame_mode_base false)
            (elif (== _output_get 1)
              (if (and (`self.IsDrawn`) (not (`NavMovementComponent.IsFalling` (`self.CharacterMovement`))))
                (`PaperZDAnimInstance.JumpToNode` (`PaperZDAnimationComponent.AnimInstance` (`self.AnimationComponent`)) "Attacking1" "None")
                (`MovementComponent.StopMovementImmediately` (`self.CharacterMovement`))
                (set `self.IsMovementLocked` true))
              (else
                (bind _asbp_cats_and_rats_2dgame_mode_base_2 (cast `/Game/Blueprints/GameMode/BP_CatsAndRats2DGameModeBase` (`GameplayStatics.GetGameMode`)))
                (`CatsAndRats2DGameModeBase.SetTransitionToNextAttack` _asbp_cats_and_rats_2dgame_mode_base_2 true)
                (`CatsAndRats2DGameModeBase.SetNextAttack` _asbp_cats_and_rats_2dgame_mode_base_2 false)))))))))

(fn `GetFeetLocation`
  (returns (ReturnValue :type "Vector Structure"))
  (bind _capsulecomponent (`self.CapsuleComponent`))
  (bind (_relativelocation_x _relativelocation_y _relativelocation_z) (`KismetMathLibrary.BreakVector` (`SceneComponent.RelativeLocation` _capsulecomponent)))
  (return (`KismetMathLibrary.MakeVector` _relativelocation_x _relativelocation_y (- _relativelocation_z (`.OutHalfHeight` (`CapsuleComponent.GetScaledCapsuleSize` _capsulecomponent))))))

(fn `UserConstructionScript`)