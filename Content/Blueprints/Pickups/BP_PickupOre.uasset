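; Ore pickup that adds its Amount to the game mode score when the hero overlaps its PickupBox.
; It shows a "+Amount" message widget, then hides itself, ignores collision on the crystal mesh and destroys the trigger box.
; It then refreshes the score in the hero's main UI and, after a short delay, removes the message and destroys itself.
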(event `self.PickupBox.OnComponentBeginOverlap`
  (params (OverlappedComponent :type "PrimitiveComponent Object Reference") (OtherActor :type "Actor Object Reference") (OtherComp :type "PrimitiveComponent Object Reference") (OtherBodyIndex :type Integer) (bFromSweep :type Boolean) (SweepResult :type "HitResult Structure (by ref)"))
  (bind _amount (`self.Amount`))
  (cast `Hero` OtherActor)
  (bind _ascats_and_rats_2dgame_mode_base (cast `CatsAndRats2DGameModeBase` (`GameplayStatics.GetGameMode`)))
  (`CatsAndRats2DGameModeBase.AddScore` _ascats_and_rats_2dgame_mode_base (`KismetMathLibrary.FTrunc` _amount))
  (bind _returnvalue (`|CreateWidget` "/Game/Blueprints/UI/Hero/WBP_MessageUserWidget.WBP_MessageUserWidget_C"))
  (set `MessageUserWidget.Message` (`KismetStringLibrary.Concat_StrStr` "+ " (`KismetStringLibrary.Conv_IntToString` (`KismetMathLibrary.FTrunc` _amount))) _returnvalue)
  (`UserWidget.AddToViewport` _returnvalue 0)
  (`self.SetActorHiddenInGame` true)
  (`PrimitiveComponent.SetCollisionResponseToAllChannels` (`self.CrystalMesh`) "ECR_Ignore")
  (`ActorComponent.K2_DestroyComponent` (`self.PickupBox`))
  (bind _asbp_hero (cast `/Game/Blueprints/Hero/BP_Hero` OtherActor))
  (bind _asbp_cats_and_rats_2dgame_mode_base (cast `/Game/Blueprints/GameMode/BP_CatsAndRats2DGameModeBase` (`GameplayStatics.GetGameMode`)))
  (`/Game/Blueprints/UI/Hero/WBP_MainUI.UpdateScore` (`/Game/Blueprints/Hero/BP_Hero.MainUIRef` _asbp_hero) (`CatsAndRats2DGameModeBase.GetCurrentScore` _asbp_cats_and_rats_2dgame_mode_base))
  (`KismetSystemLibrary.Delay` 1.0)
  (`Widget.RemoveFromParent` _returnvalue)
  (`self.K2_DestroyActor`))

(fn `UserConstructionScript`)